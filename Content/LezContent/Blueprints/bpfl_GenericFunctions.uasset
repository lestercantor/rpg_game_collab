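; A Blueprint function library of small generic helpers for mouse, book UI and item data lookups.
; CentreMouse moves the cursor to the middle of the player controller's viewport.
; CreateBookScreen spawns a Wbp_BookTesting widget for the first player with left and right page text, adds it to the viewport and returns it.
; GetItemDataTable resolves a data table row handle and returns the row when found.
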(fn CentreMouse
  (params (Player%20Controller :type Player%20Controller%20Object%20Reference))
  (bind (_sizex _sizey) (HUD|GetViewportSize Player%20Controller))
  (Class|PlayerController|SetMouseLocation Player%20Controller (/ _sizex 2) (/ _sizey 2)))

(fn CreateBookScreen
  (params (Left%20Page :type Text) (Right%20Page :type Text))
  (bind _returnvalue (UserInterface|CreateWidget "/Game/LezContent/Blueprints/TutorialBook_Blueprint/wbp_BookTesting.wbp_BookTesting_C" (Game|GetPlayerController 0) Left%20Page Right%20Page))
  (UserInterface|Viewport|AddtoViewport _returnvalue 0)
  (return _returnvalue))

(fn GetItemDataTable
  (params (ItemDataInTable :type Data%20Table%20Row%20Handle%20Structure))
  (bind _returnvalue (Utilities|GetDataTableRow (.datatable ItemDataInTable) (.rowname ItemDataInTable))
    (:then
      (return _returnvalue))))