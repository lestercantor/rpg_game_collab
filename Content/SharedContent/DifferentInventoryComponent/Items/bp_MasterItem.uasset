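; Base pickup item actor that a player interacts with to collect it into their inventory.
; The construction script sets the pickup mesh from the item's data table row, which also supplies the name for the "[E]" prompt.
; Interact finds the player's inventory component, checks its interface, sends the row name and current stack, then destroys the actor without checking whether the add succeeded.
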(event EventBeginPlay)

(event Collision|EventActorBeginOverlap
  (params (OtherActor :type Actor%20Object%20Reference)))

(event EventTick
  (params (DeltaSeconds :type Float%20%28single-precision%29)))

(event EventInteract
  (params (PlayerCharacter :type BP%20Player%20Object%20Reference))
  (bind _returnvalue (Actor|GetComponentbyClass PlayerCharacter "/Game/SharedContent/DifferentInventoryComponent/bpComponent_InventoryComponent.bpComponent_InventoryComponent_C"))
  (if (Utilities|DoesObjectImplementInterface _returnvalue "/Game/SharedContent/DifferentInventoryComponent/bpInterface_InventoryIF.bpInterface_InventoryIF_C")
    (Default|DifferentAddtoInventory _returnvalue (.rowname (Variables|Default|GetItem)) (Variables|Default|GetCurrentStack))
    (Actor|DestroyActor)))

(fn ConstructionScript
  (Components|StaticMesh|SetStaticMesh (Variables|Default|GetPickUpObject) (.ItemMesh (Utilities|Struct|Breaks_ItemStruct (CallFunction|GetItemDataTable (Variables|Default|GetItem))))))

(fn GetName
  (return (Utilities|Text|FormatText "[E] 
{item}" (.Name (Utilities|Struct|Breaks_ItemStruct (CallFunction|GetItemDataTable (Variables|Default|GetItem)))))))