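; Master pickup actor for the inventory component's items, representing an item in the world by its item ID.
; The construction script looks up the item's data table entry and sets its mesh on the PickUpObject static mesh component.
; GetName uses the same lookup to build an "[E]" prompt with the item's name.
; The event graph holds no active logic.
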(event EventBeginPlay)

(event Collision|EventActorBeginOverlap
  (params (OtherActor :type Actor%20Object%20Reference)))

(event EventTick
  (params (DeltaSeconds :type Float%20%28single-precision%29)))

(fn ConstructionScript
  (Components|StaticMesh|SetStaticMesh (Variables|Default|GetPickUpObject) (.ItemMesh (Utilities|Struct|Breaks_ItemStruct (CallFunction|GetItemDataTable (.ItemID (Utilities|Struct|BreakS_SlotStruct (Variables|Default|GetItem))))))))

(fn GetName
  (return (Utilities|Text|FormatText "[E] 
{item}" (.Name (Utilities|Struct|Breaks_ItemStruct (CallFunction|GetItemDataTable (.ItemID (Utilities|Struct|BreakS_SlotStruct (Variables|Default|GetItem)))))))))