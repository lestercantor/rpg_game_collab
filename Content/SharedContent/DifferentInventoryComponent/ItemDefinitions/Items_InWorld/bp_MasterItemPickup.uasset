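; Master world item pickup actor that lets a player collect a stack of an item into their inventory.
; The construction script sets its mesh from the item's data table row, and GetName builds an "[E]" prompt showing name and stack amount.
; On Interact, it calls TestAddToInventory on the player's inventory component after an interface check, destroying itself on success or otherwise keeping the remaining quantity.
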(event EventBeginPlay)

(event Collision|EventActorBeginOverlap
  (params (OtherActor :type Actor%20Object%20Reference)))

(event EventTick
  (params (DeltaSeconds :type Float%20%28single-precision%29)))

(event EventInteract
  (params (PlayerCharacter :type BP%20Player%20Object%20Reference))
  (bind _returnvalue (Actor|GetComponentbyClass PlayerCharacter "/Game/SharedContent/DifferentInventoryComponent/bpComponent_InventoryComponent.bpComponent_InventoryComponent_C"))
  (if (Utilities|DoesObjectImplementInterface _returnvalue "/Game/SharedContent/DifferentInventoryComponent/bpInterface_InventoryIF.bpInterface_InventoryIF_C")
    (bind (_success _quantityremaining) (Default|TestAddtoInventory _returnvalue (.rowname (Variables|Default|GetItem)) (Variables|Default|GetCurrentStack)))
    (if _success
      (Actor|DestroyActor)
      (else
        (Variables|Default|SetCurrentStack _quantityremaining)))))

(fn ConstructionScript
  (Components|StaticMesh|SetStaticMesh (Variables|Default|GetPickUpObject) (.ItemMesh (Utilities|Struct|Breaks_ItemStruct (CallFunction|GetItemDataTable (Variables|Default|GetItem))))))

(fn GetName
  (bind _item (Variables|Default|GetItem))
  (bind _itemdata (CallFunction|GetItemDataTable _item))
  (bind _name (Utilities|Struct|Breaks_ItemStruct _itemdata))
  (if (> (Variables|Default|GetCurrentStack) 1)
    (return (Utilities|Text|FormatText "[E] 
{item} ({amount})" _name (Variables|Default|GetCurrentStack)))
    (else
      (return (Utilities|Text|FormatText "[E] 
{item}" _name)))))