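; BP_Merchant is a damageable merchant character with an overhead health bar widget and an "[E]" prompt in its name.
; It forwards health, heal and damage calls to BpcDamageSystem, spawning a damage indicator actor near its torso when damaged.
; Construction Script binds the component's events: hit reactions turn it toward the player and launch it backward.
; Death ragdolls the mesh, then after a delay reattaches it to the capsule and revives it at full health.
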(event Custom|Death
  (bind _mesh (Variables|Character|GetMesh))
  (bind _mesh_2 (Variables|Character|GetMesh))
  (bind _bpc_damagesystem (Variables|Default|Getbpc_DamageSystem))
  (Development|PrintString "enemy dead")
  (Physics|SetSimulatePhysics _mesh true)
  (Collision|SetCollisionEnabled _mesh "QueryAndPhysics")
  (Utilities|FlowControl|Delay 4.0)
  (Physics|SetSimulatePhysics (Variables|Character|GetMesh) false)
  (Transformation|AttachComponentToComponent _mesh_2 (Variables|Collision|GetCapsuleComponent) "None" "SnapToTarget" "SnapToTarget" "KeepRelative" true)
  (Transformation|SetRelativeLocationAndRotation _mesh_2 "0.000000,0.000000,-100.000000" "0.000000,-90.000000,0.000000" false false)
  (Variables|/Game/SharedContent/DamageSystem/bpComponent_DamageSystem.bpComponent_DamageSystem_C|SetIsDead? _bpc_damagesystem false)
  (bind _newhealth (CallFunction|Heal (Variables|/Game/SharedContent/DamageSystem/bpComponent_DamageSystem.bpComponent_DamageSystem_C|GetMaxHealth _bpc_damagesystem)))
  (Development|PrintString (Utilities|String|ToString(Float) _newhealth)))

(event Custom|Blocked
  (params (CanBeParried :type Boolean))
  (Development|PrintString "Blocked"))

(event Custom|DamageResponse
  (params (DamageResponse :type e_DamageResponse%20Enum :default "NewEnumerator0"))
  (bind _returnvalue (Transformation|GetActorLocation))
  (bind _returnvalue_2 (Game|GetPlayerCharacter 0))
  (bind _returnvalue_3 (Transformation|GetActorLocation _returnvalue_2))
  (bind _returnvalue_4 (Math|Rotator|FindLookatRotation _returnvalue _returnvalue_3))
  (switch Utilities|FlowControl|Switch|Switchone_DamageResponse DamageResponse
    (:NewEnumerator1
      (Transformation|SetActorRotation (Math|Rotator|MakeRotator (.roll _returnvalue_4) 0.0 (.yaw _returnvalue_4)))
      (Character|LaunchCharacter (+ (* (Math|Vector|GetForwardVector (Math|Rotator|MakeRotator (.roll _returnvalue_4) 0.0 (.yaw _returnvalue_4))) -1e+02) "0.000000,0.000000,100.000000") true true)
      (Utilities|FlowControl|Delay 0.3))))

(event EventBeginPlay
  (bind _returnvalue (UserInterface|CreateWidget "/Game/SharedContent/DamageSystem/bpWidget_HealthBar.bpWidget_HealthBar_C" 0 self))
  (UserInterface|SetWidget (Variables|Default|GetHealthBarWidget) _returnvalue)
  (Variables|Default|SetLocation (Transformation|GetActorLocation)))

(fn ConstructionScript
  (bind _bpc_damagesystem (Variables|Default|Getbpc_DamageSystem))
  (EventDispatchers|BindEventtoOnDeath _bpc_damagesystem (EventDispatchers|CreateEvent :!event Custom|Death))
  (EventDispatchers|BindEventtoOnBlocked _bpc_damagesystem (EventDispatchers|CreateEvent :!event Custom|Blocked))
  (EventDispatchers|BindEventtoOnDamageResponse _bpc_damagesystem (EventDispatchers|CreateEvent :!event Custom|DamageResponse)))

(fn GetCurrentHealth
  (return (Variables|/Game/SharedContent/DamageSystem/bpComponent_DamageSystem.bpComponent_DamageSystem_C|GetHealth (Variables|Default|Getbpc_DamageSystem))))

(fn GetMaxHealth
  (return (Variables|/Game/SharedContent/DamageSystem/bpComponent_DamageSystem.bpComponent_DamageSystem_C|GetMaxHealth (Variables|Default|Getbpc_DamageSystem))))

(fn GetName
  (return (Utilities|Text|ToText(String) (Utilities|String|Append "[E] 
" (Utilities|String|ToString(Text) (Variables|Default|GetName))))))

(fn GetWeapon
  (return 0))

(fn Heal
  (params (HealAmount :type Float%20%28double-precision%29))
  (bind _new_health (Default|Heal (Variables|Default|Getbpc_DamageSystem) HealAmount))
  (return _new_health))

(fn TakeDamage
  (params (DamageInfo :type S%20Damage%20Info%20Structure))
  (bind (_wasdamaged _returnvalue) (Default|TakeDamage (Variables|Default|Getbpc_DamageSystem) DamageInfo))
  (bind (_upvector _rightvector) (Class|BpInterfacePlayer|GetVectors(Message) (Game|GetPlayerCharacter 0)))
  (Game|SpawnActorfromClass "/Game/SharedContent/DamageSystem/bp_DamageIndicator.bp_DamageIndicator_C" (Math|Transform|MakeTransform (+ (* _upvector 1e+01) (* _rightvector 1e+01) (Transformation|GetSocketLocation (Variables|Character|GetMesh) "Torso_003")) "0, 0, 0" "1.000000,1.000000,1.000000") "Undefined" "MultiplyWithRoot" 0 _returnvalue 0)
  (return _wasdamaged))