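; Base pickup item actor that a player interacts with to add it to their inventory.
; A data table row handle supplies the mesh, set in the construction script, and the name shown in an "[E]" prompt.
; Interact finds the player's inventory component, checks it implements the inventory interface, passes itself to the add function, then destroys itself without checking the result.
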(event EventBeginPlay)

(event Collision|EventActorBeginOverlap
  (params (OtherActor :type Actor%20Object%20Reference)))

(event EventTick
  (params (DeltaSeconds :type Float%20%28single-precision%29)))

(event EventInteract
  (params (PlayerCharacter :type BP%20Player%20Object%20Reference))
  (bind _returnvalue (Actor|GetComponentbyClass PlayerCharacter "/Game/SharedContent/DifferentInventoryComponent/bpComponent_InventoryComponent.bpComponent_InventoryComponent_C"))
  (if (Utilities|DoesObjectImplementInterface _returnvalue "/Game/SharedContent/DifferentInventoryComponent/bpInterface_InventoryIF.bpInterface_InventoryIF_C")
    (Default|FAddItemtoInventory _returnvalue self)
    (Actor|DestroyActor)))

(fn ConstructionScript
  (bind _item (Variables|Default|GetItem))
  (bind (_datatable _rowname) (Utilities|Struct|BreakDataTableRowHandle _item))
  (bind _returnvalue (Utilities|GetDataTableRow _datatable _rowname)
    (:then
      (Components|StaticMesh|SetStaticMesh (Variables|Default|GetPickUpObject) (.ItemMesh (Utilities|Struct|Breaks_ItemStruct _returnvalue))))))

(fn GetName
  (bind _item (Variables|Default|GetItem))
  (bind _returnvalue (Utilities|GetDataTableRow (.datatable _item) (.rowname _item))
    (:then
      (return (Utilities|Text|FormatText "[E] 
{item}" (.Name (Utilities|Struct|Breaks_ItemStruct _returnvalue)))))))