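; Floating damage-number actor that displays a damage amount in a widget and removes itself when its animation ends.
; On BeginPlay it passes the amount to its DamageIndicator widget and picks a randomized end point up and to the right, using direction vectors from the player character.
; A timeline then lerps the actor toward that point and destroys it on finish.
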(event EventBeginPlay
  (Class|BpInterfaceDamageIndicator|SetDamage(Message) (UserInterface|GetWidget (Variables|Default|GetDamageIndicator)) (Variables|Default|GetDamageIndicatorAmount))
  (bind _output_get (Variables|Default|SetStartPos (Transformation|GetActorLocation)))
  (bind (_upvector _rightvector) (Class|BpInterfacePlayer|GetVectors(Message) (Game|GetPlayerCharacter 0)))
  (Variables|Default|SetEndPos (+ _output_get (* _upvector (Math|Random|RandomFloatinRange 4e+01 5e+01)) (* _rightvector (Math|Random|RandomFloatinRange 1e+01 3e+01))))
  (bind _newtrack_0 (Timeline|DamageTimeline Play)
    (:Update
      (Transformation|SetActorLocation (Math|Vector|Lerp(Vector) (Variables|Default|GetStartPos) (Variables|Default|GetEndPos) _newtrack_0) false false))
    (:Finished
      (Actor|DestroyActor))))

(fn ConstructionScript)