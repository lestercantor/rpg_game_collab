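; Floating damage number actor that shows a damage amount and drifts away from where it spawned.
; On BeginPlay it passes DamageAmount to its bpWidget_FloatingDamageNumbers widget component.
; The MoveNumber timeline lerps the actor from its start location to a fixed raised, sideways offset, then destroys it when finished.
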(event EventBeginPlay
  (bind _asbp_widget_floating_damage_numbers (Utilities|Casting|CastTobpWidget_FloatingDamageNumbers (UserInterface|GetWidget (Variables|Default|GetDamageAmountFloatingNumber))))
  (Variables|/Game/SharedContent/DamageSystem/bpWidget_FloatingDamageNumbers.bpWidget_FloatingDamageNumbers_C|SetDamageAmount _asbp_widget_floating_damage_numbers (Variables|Default|GetDamage%20Amount))
  (bind _output_get (Variables|Default|SetStartLocation (Transformation|GetActorLocation)))
  (Variables|Default|SetEndLocation (+ _output_get "-25.000000,-25.000000,50.000000"))
  (bind _movetrack (Timeline|MoveNumber Play)
    (:Update
      (Transformation|SetActorLocation (Math|Vector|Lerp(Vector) (Variables|Default|GetStartLocation) (Variables|Default|GetEndLocation) _movetrack) false false))
    (:Finished
      (Actor|DestroyActor))))

(fn ConstructionScript)