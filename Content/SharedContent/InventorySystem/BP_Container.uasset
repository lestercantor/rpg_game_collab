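; BP_Container is an interactable world container that opens its inventory in the player's UI.
; On Interact, it casts player controller 0 to BP_FirstPersonPlayerController and passes its InventorySystem to ShowContainer on the HUD's core UI widget.
; GetName returns the container's Name prefixed with a hardcoded "[E]" key hint.
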(event EventBeginPlay)

(event Collision|EventActorBeginOverlap
  (params (OtherActor :type Actor%20Object%20Reference)))

(event EventTick
  (params (DeltaSeconds :type Float%20%28single-precision%29)))

(event EventInteract
  (params (PlayerCharacter :type BP%20Player%20Object%20Reference))
  (bind _asbp_first_person_player_controller (Utilities|Casting|CastToBP_FirstPersonPlayerController (Game|GetPlayerController 0)))
  (Default|ShowContainer (Variables|/Game/LezContent/Blueprints/bp_HUD_BaseSetup.bp_HUD_BaseSetup_C|Getwbp_Core_UI (Variables|/Game/LezContent/Blueprints/BP_FirstPersonPlayerController.BP_FirstPersonPlayerController_C|GetAs%20Bp%20HUD%20Base%20Setup _asbp_first_person_player_controller)) (Variables|Default|GetInventorySystem)))

(fn ConstructionScript)

(fn GetName
  (return (Utilities|Text|ToText(String) (Utilities|String|Append "[E] 
" (Utilities|String|ToString(Text) (Variables|Default|GetName))))))