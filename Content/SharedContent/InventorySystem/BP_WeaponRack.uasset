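; BP_WeaponRack is an interactable weapon rack that opens its inventory as a container in the player's HUD and displays stored weapons.
; Tick polls until Weapon1 is valid, looking up the rack's InventorySystem items in the Item_Data table.
; Each weapon-type item spawns its ItemClass actor, scaled up and attached to the mesh's single WeaponSlot1 socket, with only the last kept in Weapon1.
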(event Custom|ShowWeaponOnRack
  (for _array_element (Variables|/Game/SharedContent/InventorySystem/InventorySystem.InventorySystem_C|GetContent (Variables|Default|GetInventorySystem))
    (bind _returnvalue (Utilities|GetDataTableRow "/Game/SharedContent/InventorySystem/Item_Data.Item_Data" (.ItemID (Utilities|Struct|BreakFSlotStruct _array_element)))
      (:then
        (switch Utilities|FlowControl|Switch|Switchone_ItemType (.ItemType (Utilities|Struct|BreakFItemStruct _returnvalue))
          (:NewEnumerator0
            (bind _returnvalue_2 (Game|SpawnActorfromClass (.ItemClass (Utilities|Struct|BreakFItemStruct _returnvalue)) (Math|Transform|MakeTransform (Transformation|GetActorLocation) "0, 0, 0" "1.500000,1.500000,1.500000") "Undefined" "MultiplyWithRoot" 0 0))
            (bind _output_get (Variables|Default|SetWeapon1 _returnvalue_2))
            (Transformation|AttachComponentToComponent _output_get (Variables|Default|GetMesh) "WeaponSlot1" "SnapToTarget" "SnapToTarget" "KeepRelative" true)))))))

(event EventBeginPlay)

(event Collision|EventActorBeginOverlap
  (params (OtherActor :type Actor%20Object%20Reference)))

(event EventInteract
  (params (PlayerCharacter :type BP%20Player%20Object%20Reference))
  (bind _asbp_first_person_player_controller (Utilities|Casting|CastToBP_FirstPersonPlayerController (Game|GetPlayerController 0)))
  (Default|ShowContainer (Variables|/Game/LezContent/Blueprints/bp_HUD_BaseSetup.bp_HUD_BaseSetup_C|Getwbp_Core_UI (Variables|/Game/LezContent/Blueprints/BP_FirstPersonPlayerController.BP_FirstPersonPlayerController_C|GetAs%20Bp%20HUD%20Base%20Setup _asbp_first_person_player_controller)) (Variables|Default|GetInventorySystem)))

(event EventTick
  (params (DeltaSeconds :type Float%20%28single-precision%29))
  (Utilities|IsValid (Variables|Default|GetWeapon1)
    (:Is%20Not%20Valid
      (CallFunction|ShowWeapononRack))))

(fn ConstructionScript)

(fn GetName
  (return (Utilities|Text|ToText(String) (Utilities|String|Append "[E] 
" (Utilities|String|ToString(Text) (Variables|Default|GetName))))))