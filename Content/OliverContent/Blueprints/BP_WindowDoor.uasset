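; BP_WindowDoor is an interactable window door that swings open and closed when E is pressed.
; Overlapping InteractRadius shows a widget prompt for any actor, but enables input only for BP_Player, and leaving reverses this.
; A FlipFlop on E plays or reverses a timeline that lerps the door mesh's roll through a quarter turn and switches the prompt between open and close text.
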(event OnComponentBeginOverlap(InteractRadius)
  (params (OverlappedComponent :type Primitive%20Component%20Object%20Reference) (OtherActor :type Actor%20Object%20Reference) (OtherComp :type Primitive%20Component%20Object%20Reference) (OtherBodyIndex :type Integer) (bFromSweep :type Boolean) (SweepResult :type Hit%20Result%20Structure%20%28by%20ref%29))
  (Development|SetHiddeninGame (Variables|Default|GetOpenPromptText) false false)
  (Utilities|Casting|CastToBP_Player OtherActor)
  (Input|EnableInput (Game|GetPlayerController 0)))

(event OnComponentEndOverlap(InteractRadius)
  (params (OverlappedComponent :type Primitive%20Component%20Object%20Reference) (OtherActor :type Actor%20Object%20Reference) (OtherComp :type Primitive%20Component%20Object%20Reference) (OtherBodyIndex :type Integer))
  (Development|SetHiddeninGame (Variables|Default|GetOpenPromptText) true false)
  (Utilities|Casting|CastToBP_Player OtherActor)
  (Input|DisableInput (Game|GetPlayerController 0)))

(event EventBeginPlay
  (bind _asp_door_open_prompt_widget (Utilities|Casting|CastToP_DoorOpenPromptWidget (UserInterface|GetUserWidgetObject (Variables|Default|GetOpenPromptText))))
  (Variables|Default|SetInteract%20Prompt _asp_door_open_prompt_widget))

(event Input|KeyboardEvents|E
  (params (Key :type Key%20Structure))
  (bind _interact_prompt (Variables|Default|GetInteract%20Prompt))
  (:Pressed
    (Utilities|FlowControl|FlipFlop
      (:A
        (Default|UpdateText _interact_prompt "Press [E] to close")
        (bind _doorcurve (Timeline|Timeline Play)
          (:Update
            (Transformation|SetRelativeRotation (Variables|Default|GetDoorMesh) (Math|Rotator|MakeRotator (Math|Float|Lerp 0.0 -9e+01 _doorcurve) 0.0 0.0) false false))))
      (:B
        (Default|UpdateText _interact_prompt "Press [E] to open")
        (Timeline|Timeline Reverse)))))

(fn ConstructionScript)