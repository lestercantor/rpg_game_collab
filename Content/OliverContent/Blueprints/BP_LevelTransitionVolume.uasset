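; BP_LevelTransitionVolume is a trigger volume that moves the game to another level when its volume is overlapped.
; On overlap it stops the player's sprint, disables input and fades the camera out, then after a short delay async-loads ToWorld.
; When loading completes it starts a fade-in, restores input and opens the level, passing DestinationTag as options.
; GetName returns the Name prefixed with an "[E]" key label.
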(event OnComponentBeginOverlap(Volume)
  (params (OverlappedComponent :type Primitive%20Component%20Object%20Reference) (OtherActor :type Actor%20Object%20Reference) (OtherComp :type Primitive%20Component%20Object%20Reference) (OtherBodyIndex :type Integer) (bFromSweep :type Boolean) (SweepResult :type Hit%20Result%20Structure%20%28by%20ref%29))
  (bind _output_get (Variables|Default|SetPlayer%20Character (.AsBP%20Player (Utilities|Casting|CastToBP_Player (Game|GetPlayerCharacter 0)))))
  (Variables|/Game/LezContent/Blueprints/BP_Player.BP_Player_C|SetisSprinting? _output_get false)
  (Default|ResetSpeed _output_get)
  (Input|DisableInput (Variables|Default|GetPlayer%20Character) (Game|GetPlayerController 0))
  (CameraFades|StartCameraFade :self (Game|GetPlayerCameraManager 0) :ToAlpha 1.0 :Duration 0.5 :bHoldWhenFinished true)
  (Utilities|FlowControl|Delay 1.0)
  (Utilities|AsyncLoadAsset (Variables|Default|GetToWorld)
    (:Completed
      (CameraFades|StartCameraFade :self (Game|GetPlayerCameraManager 0) :FromAlpha 1.0 :Duration 0.5)
      (Input|EnableInput (Variables|Default|GetPlayer%20Character) (Game|GetPlayerController 0))
      (Game|OpenLevel(byObjectReference) (Variables|Default|GetToWorld) true (Variables|Default|GetDestinationTag)))))

(fn ConstructionScript)

(fn GetName
  (return (Utilities|Text|ToText(String) (Utilities|String|Append "[E] 
" (Utilities|String|ToString(Text) (Variables|Default|GetName))))))