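; BP_Door001 is a door that moves the player between streamed levels behind a camera fade.
; OpenDoor disables input, plays a click sound and swings the mesh slightly via a timeline.
; The timeline's Update pin, not Finished, also drives fade-out, delay, loading ToWorld, door reset, fade-in, input restore and unloading FromWorld.
; GetName exposes the door's Name variable.
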(event EventBeginPlay
  (bind _asbp_player (Utilities|Casting|CastToBP_Player (Game|GetPlayerCharacter 0)))
  (Variables|Default|SetPlayer%20Ref _asbp_player))

(event EventOpenDoor
  (Input|DisableInput (Variables|Default|GetPlayer%20Ref) (Game|GetPlayerController 0))
  (Audio|PlaySoundatLocation "/Game/SharedContent/spring-click-sound-95507.spring-click-sound-95507" (Transformation|GetWorldLocation (Variables|Default|GetDoorMesh)) "0, 0, 0" 1.0 1.0 0.0 0 0 0 0)
  (bind _doorcurve (Timeline|DoorMovementInterp PlayFromStart)
    (:Update
      (Transformation|SetRelativeRotation (Variables|Default|GetDoorMesh) (Math|Rotator|MakeRotator 0.0 0.0 (Math|Float|Lerp 0.0 -1e+01 _doorcurve)) false false)
      (CameraFades|StartCameraFade :self (Game|GetPlayerCameraManager 0) :ToAlpha 1.0 :Duration 0.5 :bHoldWhenFinished true)
      (Utilities|FlowControl|Delay 1.0)
      (Class|GameplayStatics|LoadStreamLevelbySoftObjectPtr (Variables|Default|GetToWorld) true false)
      (Transformation|SetRelativeRotation (Variables|Default|GetDoorMesh) (Math|Rotator|MakeRotator 0.0 0.0 0.0) false false)
      (CameraFades|StartCameraFade :self (Game|GetPlayerCameraManager 0) :FromAlpha 1.0 :Duration 0.5)
      (Input|EnableInput (Variables|Default|GetPlayer%20Ref) (Game|GetPlayerController 0))
      (Class|GameplayStatics|UnloadStreamLevelbySoftObjectPtr (Variables|Default|GetFromWorld) false))))

(fn ConstructionScript)

(fn GetName
  (return (Variables|Default|GetName)))